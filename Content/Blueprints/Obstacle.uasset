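; Obstacle actor for a van driving game that shifts along X each tick by the CarGameMode's Speed.
; It stops moving once the player Van's X exceeds its own.
; On root component activation it offsets its X by the game mode's TickCounter, scaled down, times Speed.
; Hitting a Van calls the Van's Collision, then disables and hides the obstacle's mesh.
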(event `self.StaticMesh.OnComponentHit`
  (params (HitComponent :type "PrimitiveComponent Object Reference") (OtherActor :type "Actor Object Reference") (OtherComp :type "PrimitiveComponent Object Reference") (NormalImpulse :type "Vector Structure") (Hit :type "HitResult Structure (by ref)"))
  (bind _staticmesh (`self.StaticMesh`))
  (bind _asvan (cast `/Game/Blueprints/Van` OtherActor))
  (`/Game/Blueprints/Van.Collision` _asvan)
  (`PrimitiveComponent.SetCollisionEnabled` _staticmesh "NoCollision")
  (`SceneComponent.SetVisibility` _staticmesh false false))

(event `self.ReceiveTick`
  (params (DeltaSeconds :type "Float (single-precision)"))
  (bind (_returnvalue_x _returnvalue_y _returnvalue_z) (`KismetMathLibrary.BreakVector` (`self.K2_GetActorLocation`)))
  (bind _returnvalue_x_2 (`KismetMathLibrary.BreakVector` (`self.K2_GetActorLocation`)))
  (if (not (`self.Stop`))
    (bind _ascar_game_mode (cast `/Game/Blueprints/CarGameMode` (`GameplayStatics.GetGameMode`)))
    (`self.K2_SetActorLocation` (`KismetMathLibrary.MakeVector` (+ (`/Game/Blueprints/CarGameMode.Speed` _ascar_game_mode) _returnvalue_x) _returnvalue_y _returnvalue_z))
    (bind _asvan (cast `/Game/Blueprints/Van` (`GameplayStatics.GetPlayerPawn` 0)))
    (bind _returnvalue_x_3 (`KismetMathLibrary.BreakVector` (`self.K2_GetActorLocation` _asvan)))
    (if (> _returnvalue_x_3 _returnvalue_x_2)
      (set `self.Stop` true))))

(event `self.DefaultSceneRoot.OnComponentActivated`
  (params (Component :type "ActorComponent Object Reference") (bReset :type Boolean))
  (bind (_returnvalue_x _returnvalue_y _returnvalue_z) (`KismetMathLibrary.BreakVector` (`self.K2_GetActorLocation`)))
  (bind _ascar_game_mode (cast `/Game/Blueprints/CarGameMode` (`GameplayStatics.GetGameMode`)))
  (`self.K2_SetActorLocation` (`KismetMathLibrary.MakeVector` (+ (* (/ (`/Game/Blueprints/CarGameMode.TickCounter` _ascar_game_mode) 100) (`/Game/Blueprints/CarGameMode.Speed` _ascar_game_mode)) _returnvalue_x) _returnvalue_y _returnvalue_z)))

(fn `UserConstructionScript`
  (set `self.Stop` false))