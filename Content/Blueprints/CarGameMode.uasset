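; Game mode for an endless driving game that builds the track from spawned tiles, starts music and the HUD, and reloads the level after death.
; Each tile's attach transform becomes the next spawn point, chaining a start tile and an initial run of floor tiles.
; A tick counter periodically drains the Van's fuel outside PillMode and raises the tile random limit, while Speed creeps up toward a cap.
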(event `PlayMusic`
  (bind _returnvalue (`AddComponent|NODE_AddAudioComponent-0`))
  (bind _output_get (set `self.AudioComponent` _returnvalue))
  (`AudioComponent.Play` _output_get 0.0))

(event `RestartGame`
  (if (`self.IsDead`)
    (`KismetSystemLibrary.Delay` 0.2)
    (bind _returnvalue (`GameplayStatics.GetCurrentLevelName` true))
    (`GameplayStatics.OpenLevel` (`KismetStringLibrary.Conv_StringToName` _returnvalue))
    (`WidgetLayoutLibrary.RemoveAllWidgets`)))

(event `self.ReceiveBeginPlay`
  (`self.PlayMusic`)
  (bind _returnvalue (`|CreateWidget` "/Game/Blueprints/HUD.HUD_C"))
  (`UserWidget.AddToViewport` _returnvalue 0)
  (`self.AddStartFloorTile`)
  (for _ (range 6)
    (`self.AddFloorTile`)))

(event `self.ReceiveTick`
  (params (DeltaSeconds :type "Float (single-precision)"))
  (bind _returnvalue (+ (`self.Speed`) 0.0005))
  (bind _result (`/Engine/EditorBlueprintResources/StandardMacros.IncrementInt` (`self.TickCounter`))
    (:`  `
      (bind _output_get (set `self.TickCounter` _result))
      (if (== (mod _output_get 300) 0)
        (bind _asvan (cast `/Game/Blueprints/Van` (`GameplayStatics.GetPlayerPawn` 0)))
        (if (not (`/Game/Blueprints/Van.PillMode` _asvan))
          (set `/Game/Blueprints/Van.Fuel` (- (`/Game/Blueprints/Van.Fuel` _asvan) 0.05) _asvan)
          (if (== (mod _output_get 1000) 0) :!label _label
            (bind _result_2 (`/Engine/EditorBlueprintResources/StandardMacros.IncrementInt` (`self.MaxTileRandomValue`))
              (:`  `
                (set `self.MaxTileRandomValue` _result_2)
                (bind _asvan_2 (cast `/Game/Blueprints/Van` (`GameplayStatics.GetPlayerPawn` 0)))
                (if (not (`/Game/Blueprints/Van.PillMode` _asvan_2))
                  (set `self.Min` 0)))))
          (if (not (>= _returnvalue 3.0))
            (set `self.Speed` _returnvalue))
          (if (>= (`self.TickCounter`) 3600)
            (set `self.TickCounter` 1)))
        (else
          (goto _label))))))

(fn `AddFloorTile`
  (bind _returnvalue (`|SpawnActorFromClass` "/Game/Blueprints/Tile.Tile_C" (`self.NextSpawnPoint`) "AlwaysSpawn" "OverrideRootScale" null null))
  (bind _astile (cast `/Game/Blueprints/Tile` _returnvalue))
  (bind _attachtransform (`/Game/Blueprints/Tile.GetAttachTransform` _astile))
  (set `self.NextSpawnPoint` _attachtransform))

(fn `AddStartFloorTile`
  (bind _returnvalue (`|SpawnActorFromClass` "/Game/Blueprints/StartTile.StartTile_C" (`KismetMathLibrary.MakeTransform` (-400.0 0.0 0.0)) "AlwaysSpawn" "OverrideRootScale" null null))
  (bind _asstart_tile (cast `/Game/Blueprints/StartTile` _returnvalue))
  (bind _attachtransform (`/Game/Blueprints/StartTile.GetAttachTransform` _asstart_tile))
  (set `self.NextSpawnPoint` _attachtransform))

(fn `ReturnPlayerPawn`
  (returns (ReturnValue :type "Pawn Object Reference"))
  (return (`GameplayStatics.GetPlayerPawn` 0)))

(fn `UserConstructionScript`)