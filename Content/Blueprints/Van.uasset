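; Player van pawn for a three-lane endless runner that drives forward automatically and hops sideways on Left/Right input.
; Applies the car material chosen in CarGameMode and spins its axles with velocity.
; Pills trigger a timed speed boost with altered saturation, during which collisions wreck cars instead of costing lives.
; Running out of lives or fuel hides and freezes the van, then flags death in the game mode.
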(event `SetCar`
  (`KismetSystemLibrary.Delay` 0.01)
  (bind _ascar_game_mode (cast `/Game/Blueprints/CarGameMode` (`GameplayStatics.GetGameMode`)))
  (switch `int` (`/Game/Blueprints/CarGameMode.ChosenCar` _ascar_game_mode)
    (:`0`
      (set `self.CarMat` "/Game/Materials/van.van"))
    (:`1`
      (set `self.CarMat` "/Game/Materials/pill1.pill1"))
    (:`2`
      (set `self.CarMat` "/Game/Materials/pill2.pill2"))
    (:`3`
      (set `self.CarMat` "/Game/Materials/grass.grass"))
    (:`4`
      (set `self.CarMat` "/Game/Materials/metal2.metal2")))
  (`PrimitiveComponent.SetMaterial` (`self.Van`) 0 (`self.CarMat`)))

(event `GetPill`
  (bind _floatingpawnmovement (`self.FloatingPawnMovement`))
  (if (not (`self.PillMode`))
    (set `CameraComponent.PostProcessSettings` (make `PostProcessSettings` :`ColorSaturation` (`self.Saturation`)) (`self.Camera`))
    (set `FloatingPawnMovement.MaxSpeed` 2000.0 _floatingpawnmovement)
    (set `FloatingPawnMovement.Acceleration` 5000.0 _floatingpawnmovement)
    (bind _result (`/Engine/EditorBlueprintResources/StandardMacros.IncrementInt` (`self.TotalPills`))
      (:`  `
        (set `self.TotalPills` _result)
        (set `self.PillMode` true)
        (bind _ascar_game_mode (cast `/Game/Blueprints/CarGameMode` (`GameplayStatics.GetGameMode`)))
        (set `/Game/Blueprints/CarGameMode.Min` 1 _ascar_game_mode)
        (bind _audiocomponent (`/Game/Blueprints/CarGameMode.AudioComponent` _ascar_game_mode))
        (`AudioComponent.SetPaused` _audiocomponent true)
        (`GameplayStatics.PlaySound2D` "/Game/Audio/get_pill_Cue.get_pill_Cue" 1.0 1.0 0.0 null null)
        (`KismetSystemLibrary.Delay` 27.0)
        (set `FloatingPawnMovement.MaxSpeed` 1000.0 _floatingpawnmovement)
        (`KismetSystemLibrary.Delay` 3.0)
        (`AudioComponent.SetPaused` _audiocomponent false)
        (set `FloatingPawnMovement.Acceleration` 50.0 _floatingpawnmovement)
        (set `self.PillMode` false)
        (set `CameraComponent.PostProcessSettings` (`self.DefaultPostProcessSettings`) (`self.Camera`))))))

(event `self.ReceiveBeginPlay`
  (bind _audiocomponent (`self.AudioComponent`))
  (`self.SetCar`)
  (set `self.DefaultPostProcessSettings` (`CameraComponent.PostProcessSettings` (`self.Camera`)))
  (bind _returnvalue (`AddComponent|NODE_AddAudioComponent-0`))
  (bind _output_get (set `self.AudioComponent` _returnvalue))
  (`AudioComponent.Play` _output_get 0.0)
  (`KismetSystemLibrary.Delay` 1.0)
  (`AudioComponent.SetSound` _audiocomponent "/Game/Audio/engine_Cue.engine_Cue")
  (`AudioComponent.Play` _audiocomponent 0.0))

(event `Collision`
  (if (`self.PillMode`)
    (`GameplayStatics.PlaySound2D` "/Game/Audio/crush_Cue.crush_Cue" 1.0 1.0 0.0 null null)
    (bind _result (`/Engine/EditorBlueprintResources/StandardMacros.IncrementInt` (`self.TotalCarsWrecked`))
      (:`  `
        (set `self.TotalCarsWrecked` _result)))
    (else
      (`self.RemoveLife`)
      (if (<= (`self.Lifes`) 0)
        (`GameplayStatics.PlaySound2D` "/Game/Audio/game_over_Cue.game_over_Cue" 1.0 1.0 0.0 null null)
        (`AudioComponent.Stop` (`self.AudioComponent`) :!label _label)
        (`self.DisableInput` null)
        (`SceneComponent.SetVisibility` (`self.van`) false false)
        (`SceneComponent.SetVisibility` (`self.Axis1`) false false)
        (`SceneComponent.SetVisibility` (`self.wheel1`) false false)
        (`SceneComponent.SetVisibility` (`self.wheel2`) false false)
        (`SceneComponent.SetVisibility` (`self.Axis2`) false false)
        (`SceneComponent.SetVisibility` (`self.wheel3`) false false)
        (`SceneComponent.SetVisibility` (`self.wheel4`) false false)
        (set `self.DeathLocation` (`self.K2_GetActorLocation`))
        (set `self.Lifes` -1)
        (`KismetSystemLibrary.Delay` 0.25)
        (set `self.Lifes` -2)
        (bind _ascar_game_mode (cast `/Game/Blueprints/CarGameMode` (`GameplayStatics.GetGameMode`)))
        (set `/Game/Blueprints/CarGameMode.IsDead` true _ascar_game_mode)
        (else
          (`GameplayStatics.PlaySound2D` "/Game/Audio/crush2_Cue.crush2_Cue" 1.0 1.0 0.0 null null))))))

(event `self.ReceiveTick`
  (params (DeltaSeconds :type "Float (single-precision)"))
  (bind _returnvalue_x (`KismetMathLibrary.BreakVector` (`self.GetVelocity`)))
  (bind (_returnvalue_x_2 _returnvalue_y _returnvalue_z) (`KismetMathLibrary.BreakVector` (`self.K2_GetActorLocation`)))
  (if (<= (`self.Fuel`) 0.0)
    (goto _label)
    (else
      (if (> _returnvalue_z 25.125)
        (`self.K2_SetActorLocation` (`KismetMathLibrary.MakeVector` _returnvalue_x_2 _returnvalue_y 25.125)))
      (bind _ascar_game_mode (cast `/Game/Blueprints/CarGameMode` (`GameplayStatics.GetGameMode`)))
      (bind _returnvalue (* (`/Game/Blueprints/CarGameMode.TickCounter` _ascar_game_mode) (/ _returnvalue_x -250.0)))
      (`SceneComponent.K2_SetRelativeRotation` (`self.Axis1`) (`KismetMathLibrary.MakeRotator` 0.0 _returnvalue) false false)
      (`SceneComponent.K2_SetRelativeRotation` (`self.Axis2`) (`KismetMathLibrary.MakeRotator` 0.0 _returnvalue) false false)
      (if (<= (`self.Lifes`) 0)
        (`self.K2_SetActorLocation` (`self.DeathLocation`))
        (else
          (`self.AddMovementInput` (`KismetMathLibrary.GetForwardVector` (`KismetMathLibrary.MakeRotator` 0.0 0.0 (.yaw (`self.GetControlRotation`))))))))))

(event `GetCanister`
  (`GameplayStatics.PlaySound2D` "/Game/Audio/fuel_Cue.fuel_Cue" 1.0 1.0 0.0 null null)
  (set `self.Fuel` 1.0))

(event `InputAction|Left`
  (params (Key :type "Key Structure"))
  (bind (_returnvalue_x _returnvalue_y) (`KismetMathLibrary.BreakVector` (`self.K2_GetActorLocation`)))
  (bind _camera (`self.Camera`))
  (bind (_returnvalue_x_2 _returnvalue_y_2 _returnvalue_z) (`KismetMathLibrary.BreakVector` (`SceneComponent.K2_GetComponentLocation` _camera)))
  (:`Pressed`
    (if (== _returnvalue_y 0.0)
      (bind (_sweephitresult _returnvalue) (`self.K2_SetActorLocation` (`KismetMathLibrary.MakeVector` _returnvalue_x -60.0 25.125) true))
      (if _returnvalue
        (`self.K2_SetActorLocation` (`KismetMathLibrary.MakeVector` _returnvalue_x -60.0 25.125) true))
      (else
        (bind (_sweephitresult_2 _returnvalue_2) (`self.K2_SetActorLocation` (`KismetMathLibrary.MakeVector` _returnvalue_x 0.0 25.125) true))
        (if _returnvalue_2
          (`self.K2_SetActorLocation` (`KismetMathLibrary.MakeVector` _returnvalue_x 0.0 25.125) true))))
    (`SceneComponent.K2_SetWorldLocation` _camera (`KismetMathLibrary.MakeVector` _returnvalue_x_2 0.0 _returnvalue_z) false false)))

(event `InputAction|Right`
  (params (Key :type "Key Structure"))
  (bind (_returnvalue_x _returnvalue_y) (`KismetMathLibrary.BreakVector` (`self.K2_GetActorLocation`)))
  (bind _camera (`self.Camera`))
  (bind (_returnvalue_x_2 _returnvalue_y_2 _returnvalue_z) (`KismetMathLibrary.BreakVector` (`SceneComponent.K2_GetComponentLocation` _camera)))
  (:`Pressed`
    (if (== _returnvalue_y 0.0)
      (bind (_sweephitresult _returnvalue) (`self.K2_SetActorLocation` (`KismetMathLibrary.MakeVector` _returnvalue_x 60.0 25.125) true))
      (if _returnvalue
        (`self.K2_SetActorLocation` (`KismetMathLibrary.MakeVector` _returnvalue_x 60.0 25.125) true))
      (else
        (bind (_sweephitresult_2 _returnvalue_2) (`self.K2_SetActorLocation` (`KismetMathLibrary.MakeVector` _returnvalue_x 0.0 25.125) true))
        (if _returnvalue_2
          (`self.K2_SetActorLocation` (`KismetMathLibrary.MakeVector` _returnvalue_x 0.0 25.125) true))))
    (`SceneComponent.K2_SetWorldLocation` _camera (`KismetMathLibrary.MakeVector` _returnvalue_x_2 0.0 _returnvalue_z) false false)))

(fn `AddItem`
  (set `self.TotalItems` (+ (`self.TotalItems`) 1))
  (`GameplayStatics.PlaySound2D` "/Game/Audio/point_Cue.point_Cue" 1.0 1.0 0.0 null null))

(fn `RemoveLife`
  (set `self.Lifes` (- (`self.Lifes`) 1)))

(fn `UserConstructionScript`)