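; Car1 is a car actor that the player's CarGamePawn can crash into, with a body mesh, two axles and four wheels.
; The construction script randomly picks one of four metal materials for the body.
; Each tick it runs the parent tick and spins both axles from CarGameMode's TickCounter.
; When the pawn hits the body, it calls the pawn's Collision, then hides the car's parts and disables their collision.
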(event `self.StaticMesh.OnComponentHit`
  (params (HitComponent :type "PrimitiveComponent Object Reference") (OtherActor :type "Actor Object Reference") (OtherComp :type "PrimitiveComponent Object Reference") (NormalImpulse :type "Vector Structure") (Hit :type "HitResult Structure (by ref)"))
  (bind _asvan (cast `/Game/Blueprints/CarGamePawn` OtherActor))
  (`/Game/Blueprints/CarGamePawn.Collision` _asvan)
  (`PrimitiveComponent.SetCollisionEnabled` (`self.car1_wheel1`) "NoCollision")
  (`PrimitiveComponent.SetCollisionEnabled` (`self.car1_wheel2`) "NoCollision")
  (`PrimitiveComponent.SetCollisionEnabled` (`self.Axis1`) "NoCollision")
  (`PrimitiveComponent.SetCollisionEnabled` (`self.car1_wheel3`) "NoCollision")
  (`PrimitiveComponent.SetCollisionEnabled` (`self.car1_wheel4`) "NoCollision")
  (`PrimitiveComponent.SetCollisionEnabled` (`self.Axis2`) "NoCollision")
  (`PrimitiveComponent.SetCollisionEnabled` (`self.StaticMesh`) "NoCollision")
  (`SceneComponent.SetVisibility` (`self.Axis2`) false false)
  (`SceneComponent.SetVisibility` (`self.car1_wheel4`) false false)
  (`SceneComponent.SetVisibility` (`self.car1_wheel3`) false false)
  (`SceneComponent.SetVisibility` (`self.Axis1`) false false)
  (`SceneComponent.SetVisibility` (`self.car1_wheel2`) false false)
  (`SceneComponent.SetVisibility` (`self.car1_wheel1`) false false)
  (`SceneComponent.SetVisibility` (`self.StaticMesh`) false false))

(event `self.ReceiveTick`
  (params (DeltaSeconds :type "Float (single-precision)"))
  (`parent.ReceiveTick` 0.0)
  (bind _ascar_game_mode (cast `/Game/Blueprints/CarGameMode` (`GameplayStatics.GetGameMode`)))
  (bind _returnvalue (* (`/Game/Blueprints/CarGameMode.TickCounter` _ascar_game_mode) -10.0))
  (`SceneComponent.K2_SetRelativeRotation` (`self.Axis1`) (`KismetMathLibrary.MakeRotator` 0.0 _returnvalue) false false)
  (`SceneComponent.K2_SetRelativeRotation` (`self.Axis2`) (`KismetMathLibrary.MakeRotator` 0.0 _returnvalue) false false))

(fn `UserConstructionScript`
  (bind _staticmesh (`self.StaticMesh`))
  (`parent.UserConstructionScript`)
  (switch `int` (`KismetMathLibrary.RandomIntegerInRange` 0 4)
    (:`Default`
      (`PrimitiveComponent.SetMaterial` _staticmesh 0 "/Game/Materials/metal1.metal1" :!label _label))
    (:`0`
      (goto _label))
    (:`1`
      (`PrimitiveComponent.SetMaterial` _staticmesh 0 "/Game/Materials/metal2.metal2"))
    (:`2`
      (`PrimitiveComponent.SetMaterial` _staticmesh 0 "/Game/Materials/metal3.metal3"))
    (:`3`
      (`PrimitiveComponent.SetMaterial` _staticmesh 0 "/Game/Materials/metal4.metal4"))))