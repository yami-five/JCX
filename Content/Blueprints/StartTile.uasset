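; StartTile is a floor tile actor for an endless driving game.
; When a Van overlaps its end trigger, it asks CarGameMode to add a floor tile, then destroys itself after a delay.
; Helper functions expose the attach transform for chaining tiles, gather three relative spawn point transforms and pick one of three item areas at random.
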(event `self.EndTrigger.OnComponentBeginOverlap`
  (params (OverlappedComponent :type "PrimitiveComponent Object Reference") (OtherActor :type "Actor Object Reference") (OtherComp :type "PrimitiveComponent Object Reference") (OtherBodyIndex :type Integer) (bFromSweep :type Boolean) (SweepResult :type "HitResult Structure (by ref)"))
  (cast `/Game/Blueprints/Van` OtherActor)
  (bind _ascar_game_mode (cast `/Game/Blueprints/CarGameMode` (`GameplayStatics.GetGameMode`)))
  (`/Game/Blueprints/CarGameMode.AddFloorTile` _ascar_game_mode)
  (`KismetSystemLibrary.Delay` 20.0)
  (`self.K2_DestroyActor`))

(fn `DrawItemArea`
  (returns (ItemArea :type "BoxComponent Object Reference"))
  (switch `int` (`KismetMathLibrary.RandomIntegerInRange` 0 2)
    (:`0`
      (bind _output_get (set `self.Area` (`self.ItemArea`)))
      (return _output_get))
    (:`1`
      (bind _output_get_2 (set `self.Area` (`self.ItemAreaL`)))
      (return _output_get_2))
    (:`2`
      (bind _output_get_3 (set `self.Area` (`self.ItemAreaR`)))
      (return _output_get_3))))

(fn `GetAttachTransform`
  (returns (AttachTransform :type "Transform Structure"))
  (return (`SceneComponent.K2_GetComponentToWorld` (`self.AttachPoint`))))

(fn `GetSpawnPoints`
  (set `self.SpawnPoints` (`|MakeArray` (`SceneComponent.GetRelativeTransform` (`self.SpawnPointR`)) (`SceneComponent.GetRelativeTransform` (`self.SpawnPointL`)) (`SceneComponent.GetRelativeTransform` (`self.SpawnPoint`)))))

(fn `UserConstructionScript`)