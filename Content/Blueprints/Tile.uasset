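; Endless-runner floor tile for the Van, exposing an attach transform and filled with random content on construction.
; Construction may place an obstacle at one of three spawn points, with odds shaped by CarGameMode.
; It also spawns items, a pill, or occasionally a canister when fuel is low, randomly inside one of three box areas.
; When the Van hits EndTrigger, CarGameMode adds another tile and this one destroys itself after a delay.
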(event `self.EndTrigger.OnComponentBeginOverlap`
  (params (OverlappedComponent :type "PrimitiveComponent Object Reference") (OtherActor :type "Actor Object Reference") (OtherComp :type "PrimitiveComponent Object Reference") (OtherBodyIndex :type Integer) (bFromSweep :type Boolean) (SweepResult :type "HitResult Structure (by ref)"))
  (cast `/Game/Blueprints/Van` OtherActor)
  (bind _ascar_game_mode (cast `/Game/Blueprints/CarGameMode` (`GameplayStatics.GetGameMode`)))
  (`/Game/Blueprints/CarGameMode.AddFloorTile` _ascar_game_mode)
  (`KismetSystemLibrary.Delay` 20.0)
  (`self.K2_DestroyActor`))

(fn `DrawItemArea`
  (returns (ItemArea :type "BoxComponent Object Reference"))
  (switch `int` (`KismetMathLibrary.RandomIntegerInRange` 0 2)
    (:`0`
      (bind _output_get (set `self.Area` (`self.ItemArea`)))
      (return _output_get))
    (:`1`
      (bind _output_get_2 (set `self.Area` (`self.ItemAreaL`)))
      (return _output_get_2))
    (:`2`
      (bind _output_get_3 (set `self.Area` (`self.ItemAreaR`)))
      (return _output_get_3))))

(fn `GetAttachTransform`
  (returns (AttachTransform :type "Transform Structure"))
  (return (`SceneComponent.K2_GetComponentToWorld` (`self.AttachPoint`))))

(fn `GetSpawnPoints`
  (set `self.SpawnPoints` (`|MakeArray` (`SceneComponent.GetRelativeTransform` (`self.SpawnPointR`)) (`SceneComponent.GetRelativeTransform` (`self.SpawnPointL`)) (`SceneComponent.GetRelativeTransform` (`self.SpawnPoint`)))))

(fn `Spawn Obstacle`
  (bind _spawnpoints (`self.SpawnPoints`))
  (`AddComponent|NODE_AddChildActorComponent-0` :`RelativeTransform` (`|GetArrayItem` _spawnpoints (`KismetMathLibrary.RandomIntegerInRange` 0 (`KismetArrayLibrary.Array_LastIndex` _spawnpoints)))))

(fn `SpawnCanister`
  (bind _itemarea (`self.DrawItemArea`))
  (`AddComponent|NODE_AddChildActorComponent-3` :`RelativeTransform` (`KismetMathLibrary.Conv_VectorToTransform` (`KismetMathLibrary.RandomPointInBoundingBox` (`SceneComponent.RelativeLocation` _itemarea) (`BoxComponent.BoxExtent` _itemarea)))))

(fn `SpawnItem`
  (bind _itemarea (`self.DrawItemArea`))
  (for _ (range 2)
    (`AddComponent|NODE_AddChildActorComponent-1` :`RelativeTransform` (`KismetMathLibrary.Conv_VectorToTransform` (`KismetMathLibrary.RandomPointInBoundingBox` (`SceneComponent.RelativeLocation` _itemarea) (`BoxComponent.BoxExtent` _itemarea))))))

(fn `SpawnPill`
  (bind _itemarea (`self.DrawItemArea`))
  (`AddComponent|NODE_AddChildActorComponent-2` :`RelativeTransform` (`KismetMathLibrary.Conv_VectorToTransform` (`KismetMathLibrary.RandomPointInBoundingBox` (`SceneComponent.RelativeLocation` _itemarea) (`BoxComponent.BoxExtent` _itemarea)))))

(fn `UserConstructionScript`
  (`self.GetSpawnPoints`)
  (bind _ascar_game_mode (cast `/Game/Blueprints/CarGameMode` (`GameplayStatics.GetGameMode`)))
  (switch `int` (`KismetMathLibrary.RandomIntegerInRange` 0 (`/Game/Blueprints/CarGameMode.MaxTileRandomValue` _ascar_game_mode))
    (:`Default`
      (`self.Spawn Obstacle` :!label _label))
    (:`0`
      _)
    (:`1`
      (goto _label))
    (:`2`
      _)
    (:`3`
      _)
    (:`4`
      (goto _label))
    (:`5`
      (goto _label))
    (:`6`
      _))
  (switch `int` (`KismetMathLibrary.RandomIntegerInRange` (`/Game/Blueprints/CarGameMode.Min` _ascar_game_mode) 100)
    (:`Default`
      (bind _returnvalue (`/Game/Blueprints/CarGameMode.ReturnPlayerPawn` _ascar_game_mode))
      (bind _asvan (cast `/Game/Blueprints/Van` _returnvalue))
      (if (<= (`/Game/Blueprints/Van.Fuel` _asvan) 0.5)
        (switch `int` (`KismetMathLibrary.RandomIntegerInRange` 0 20)
          (:`Default`
            (`self.SpawnItem` :!label _label_2))
          (:`0`
            (`self.SpawnCanister`)))
        (else
          (goto _label_2))))
    (:`0`
      (`self.SpawnPill`))))