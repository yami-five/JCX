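; CarMenuController handles confirming or cancelling car selection in the car menu, persisting the choice in the "CarSave" slot.
; On BeginPlay it loads any existing save and restores the CarMenuPawn's cursor to the saved ChosenCar.
; Start writes the pawn's cursor position to a newly created CarSaveGame, saves it, then opens MainMenu.
; Escape opens MainMenu without saving.
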(event `self.ReceiveBeginPlay`
  (bind _returnvalue (`GameplayStatics.DoesSaveGameExist` "CarSave"))
  (if _returnvalue
    (bind _returnvalue_2 (`GameplayStatics.LoadGameFromSlot` "CarSave"))
    (bind _ascar_save_game (cast `/Game/Blueprints/CarSaveGame` _returnvalue_2))
    (bind _ascar_menu_pawn (cast `/Game/Blueprints/MainMenuBluprints/CarMenuPawn` (`GameplayStatics.GetPlayerPawn` 0)))
    (set `/Game/Blueprints/MainMenuBluprints/CarMenuPawn.CursorPosition` (`/Game/Blueprints/CarSaveGame.ChosenCar` _ascar_save_game) _ascar_menu_pawn)))

(event `InputAction|Start`
  (params (Key :type "Key Structure"))
  (:`Pressed`
    (bind _returnvalue (`GameplayStatics.CreateSaveGameObject` "/Game/Blueprints/CarSaveGame.CarSaveGame_C"))
    (bind _output_get (set `self.Save_Ref` _returnvalue))
    (bind _ascar_menu_pawn (cast `/Game/Blueprints/MainMenuBluprints/CarMenuPawn` (`GameplayStatics.GetPlayerPawn` 0)))
    (set `/Game/Blueprints/CarSaveGame.ChosenCar` (`/Game/Blueprints/MainMenuBluprints/CarMenuPawn.CursorPosition` _ascar_menu_pawn) _output_get)
    (`GameplayStatics.SaveGameToSlot` _output_get "CarSave")
    (`GameplayStatics.OpenLevel` "MainMenu" :!label _label)))

(event `InputAction|Escape`
  (params (Key :type "Key Structure"))
  (:`Pressed`
    (goto _label)))

(fn `UserConstructionScript`)