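; Main menu mode that loads or creates the CarSave slot, caching the chosen car and lifetime stats.
; On loading an existing save, UnlockVans flags at most one locked van whose bottle, pill, high score or crash threshold is met, leaving disk writes to SaveData.
; Events show and close the Stats widget.
; Tick runs a frame counter that wraps at 360.
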(event `SaveData`
  (`GameplayStatics.SaveGameToSlot` (`self.SaveRef`) "CarSave"))

(event `self.ReceiveBeginPlay`
  (bind _stats (`self.Stats`))
  (bind _returnvalue (`GameplayStatics.DoesSaveGameExist` "CarSave"))
  (if _returnvalue
    (bind _returnvalue_2 (`GameplayStatics.LoadGameFromSlot` "CarSave"))
    (bind _ascar_save_game (cast `/Game/Blueprints/CarSaveGame` _returnvalue_2))
    (bind _output_get (set `self.SaveRef` _ascar_save_game))
    (set `self.ChosenCar` (`/Game/Blueprints/CarSaveGame.ChosenCar` _output_get))
    (bind _highscore (`/Game/Blueprints/CarSaveGame.HighScore` _output_get))
    (`KismetArrayLibrary.Array_Set` _stats 0 _highscore)
    (bind _totalpillsnum (`/Game/Blueprints/CarSaveGame.TotalPillsNum` _output_get))
    (`KismetArrayLibrary.Array_Set` _stats 2 _totalpillsnum)
    (bind _totalbottlesnum (`/Game/Blueprints/CarSaveGame.TotalBottlesNum` _output_get))
    (`KismetArrayLibrary.Array_Set` _stats 1 _totalbottlesnum)
    (bind _crashedcars (`/Game/Blueprints/CarSaveGame.CrashedCars` _output_get))
    (`KismetArrayLibrary.Array_Set` _stats 3 _crashedcars)
    (`self.UnlockVans` _output_get)
    (if (`self.Debug`)
      (`KismetSystemLibrary.PrintString` (`KismetStringLibrary.Conv_IntToString` _highscore))
      (`KismetSystemLibrary.PrintString` (`KismetStringLibrary.Conv_IntToString` _totalpillsnum))
      (`KismetSystemLibrary.PrintString` (`KismetStringLibrary.Conv_IntToString` _totalbottlesnum))
      (`KismetSystemLibrary.PrintString` (`KismetStringLibrary.Conv_IntToString` _crashedcars)))
    (else
      (bind _returnvalue_3 (`GameplayStatics.CreateSaveGameObject` "/Game/Blueprints/CarSaveGame.CarSaveGame_C"))
      (bind _ascar_save_game_2 (cast `/Game/Blueprints/CarSaveGame` _returnvalue_3))
      (bind _output_get_2 (set `self.SaveRef` _ascar_save_game_2))
      (`GameplayStatics.SaveGameToSlot` _output_get_2 "CarSave"))))

(event `self.ReceiveTick`
  (params (DeltaSeconds :type "Float (single-precision)"))
  (bind _result (`/Engine/EditorBlueprintResources/StandardMacros.IncrementInt` (`self.TickCounter`))
    (:`  `
      (bind _output_get (set `self.TickCounter` _result))
      (if (== _output_get 360)
        (set `self.TickCounter` 0)))))

(event `ShowStats`
  (set `self.ShowingStats` true)
  (bind _returnvalue (`|CreateWidget` "/Game/Blueprints/MainMenuBluprints/Stats.Stats_C"))
  (`UserWidget.AddToViewport` _returnvalue 0))

(event `CloseStats`
  (set `self.ShowingStats` false)
  (bind _foundwidgets (`WidgetBlueprintLibrary.GetAllWidgetsOfClass` "/Game/Blueprints/MainMenuBluprints/Stats.Stats_C"))
  (`Widget.RemoveFromParent` _foundwidgets))

(fn `UnlockVans`
  (params (SaveRefIn :type "/Game/Blueprints/CarSaveGame Object Reference"))
  (bind _vans (`/Game/Blueprints/CarSaveGame.Vans` SaveRefIn))
  (for (_array_element _array_index) _vans
    (if (not _array_element)
      (switch `int` _array_index
        (:`0`
          (if (>= (`/Game/Blueprints/CarSaveGame.TotalBottlesNum` SaveRefIn) 1000)
            (`KismetArrayLibrary.Array_Set` _vans _array_index true :!label _label)
            (return)))
        (:`1`
          (if (>= (`/Game/Blueprints/CarSaveGame.TotalPillsNum` SaveRefIn) 10)
            (goto _label)))
        (:`2`
          (if (>= (`/Game/Blueprints/CarSaveGame.HighScore` SaveRefIn) 100000)
            (goto _label)))
        (:`3`
          (if (>= (`/Game/Blueprints/CarSaveGame.CrashedCars` SaveRefIn) 100)
            (goto _label))))))
  (return))

(fn `UserConstructionScript`)