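; MenuCar is a car actor for the main menu that shows the player's chosen car look on its Van mesh.
; Shortly after BeginPlay, it checks the game mode by object name, then maps MainMenuMode's ChosenCar to one of five materials for the mesh's first slot.
; Any other game mode just gets its name printed.
; Logic to rotate Axis1 from the mode's TickCounter is present but unconnected, and Tick is empty.
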(event `self.ReceiveBeginPlay`
  (bind _returnvalue (`GameplayStatics.GetGameMode`))
  (bind _returnvalue_2 (`KismetSystemLibrary.GetObjectName` _returnvalue))
  (`KismetSystemLibrary.Delay` 0.01)
  (if (`KismetStringLibrary.EqualEqual_StrStr` _returnvalue_2 "MainMenuMode_C_0")
    (bind _asmain_menu_mode (cast `/Game/Blueprints/MainMenuBluprints/MainMenuMode` _returnvalue))
    (switch `int` (`/Game/Blueprints/MainMenuBluprints/MainMenuMode.ChosenCar` _asmain_menu_mode)
      (:`0`
        (set `self.CarMat` "/Game/Materials/van.van"))
      (:`1`
        (set `self.CarMat` "/Game/Materials/pill1.pill1"))
      (:`2`
        (set `self.CarMat` "/Game/Materials/pill2.pill2"))
      (:`3`
        (set `self.CarMat` "/Game/Materials/grass.grass"))
      (:`4`
        (set `self.CarMat` "/Game/Materials/metal2.metal2")))
    (`PrimitiveComponent.SetMaterial` (`self.Van`) 0 (`self.CarMat`))
    (else
      (`KismetSystemLibrary.PrintString` _returnvalue_2))))

(event `self.ReceiveTick`
  (params (DeltaSeconds :type "Float (single-precision)")))

(fn `UserConstructionScript`)