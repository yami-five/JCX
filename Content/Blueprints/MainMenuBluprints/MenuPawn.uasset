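; MenuPawn is a main menu pawn that moves a cursor component between three button components using Up and Down input.
; On BeginPlay it stores the three buttons' relative locations in an array and places the cursor at the first one's height.
; Up and Down presses step a cursor index with wraparound, then set the cursor's relative Z to that button's stored Z, leaving X and Y unchanged.
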(event `self.ReceiveBeginPlay`
  (bind _buttonspositions (`self.ButtonsPositions`))
  (bind _cursor (`self.Cursor`))
  (bind (_output_x _output_y _output_z) (`KismetMathLibrary.BreakVector` (`|GetArrayItem` (`self.ButtonsPositions`))))
  (bind (_relativelocation_x _relativelocation_y) (`KismetMathLibrary.BreakVector` (`SceneComponent.RelativeLocation` _cursor)))
  (`KismetArrayLibrary.Array_Set` _buttonspositions 0 (`SceneComponent.RelativeLocation` (`self.Button1`)))
  (`KismetArrayLibrary.Array_Set` _buttonspositions 1 (`SceneComponent.RelativeLocation` (`self.Button2`)))
  (`KismetArrayLibrary.Array_Set` _buttonspositions 2 (`SceneComponent.RelativeLocation` (`self.Button3`)))
  (`SceneComponent.K2_SetRelativeLocation` _cursor (`KismetMathLibrary.MakeVector` _relativelocation_x _relativelocation_y _output_z) false false))

(event `InputAction|Up`
  (params (Key :type "Key Structure"))
  (bind _cursor (`self.Cursor`))
  (bind _cursorposition (`self.CursorPosition`))
  (bind (_output_x _output_y _output_z) (`KismetMathLibrary.BreakVector` (`|GetArrayItem` (`self.ButtonsPositions`) _cursorposition)))
  (bind (_relativelocation_x _relativelocation_y) (`KismetMathLibrary.BreakVector` (`SceneComponent.RelativeLocation` _cursor)))
  (:`Pressed`
    (bind _output_get (set `self.CursorPosition` (- _cursorposition 1)))
    (if (< _output_get 0)
      (set `self.CursorPosition` 2))
    (`SceneComponent.K2_SetRelativeLocation` _cursor (`KismetMathLibrary.MakeVector` _relativelocation_x _relativelocation_y _output_z) false false :!label _label)))

(event `InputAction|Down`
  (params (Key :type "Key Structure"))
  (:`Pressed`
    (bind _result (`/Engine/EditorBlueprintResources/StandardMacros.IncrementInt` (`self.CursorPosition`))
      (:`  `
        (bind _output_get (set `self.CursorPosition` _result))
        (if (> _output_get 2)
          (set `self.CursorPosition` 0)
          (goto _label)
          (else
            (goto _label)))))))

(fn `UserConstructionScript`)