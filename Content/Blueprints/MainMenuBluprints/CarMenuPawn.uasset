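; CarMenuPawn is the car selection menu pawn that scrolls a camera along a list of cars.
; Left and Right inputs play a menu sound, tell CarMenuMode to redraw its widget, and step a cursor that wraps across five slots.
; On BeginPlay and after each step, the camera snaps its relative Y to the selected car's world Y, keeping X and Z.
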(event `self.ReceiveBeginPlay`
  (bind _camera (`self.Camera`))
  (bind (_relativelocation_x _relativelocation_y _relativelocation_z) (`KismetMathLibrary.BreakVector` (`SceneComponent.RelativeLocation` _camera)))
  (bind (_returnvalue_x _returnvalue_y) (`KismetMathLibrary.BreakVector` (`self.K2_GetActorLocation` (`|GetArrayItem` (`self.CarsList`) (`self.CursorPosition`)))))
  (`SceneComponent.K2_SetRelativeLocation` _camera (`KismetMathLibrary.MakeVector` _relativelocation_x _returnvalue_y _relativelocation_z) false false :!label _label))

(event `InputAction|Left`
  (params (Key :type "Key Structure"))
  (:`Pressed`
    (bind _ascar_menu_mode (cast `/Game/Blueprints/MainMenuBluprints/CarMenuMode` (`GameplayStatics.GetGameMode`)))
    (`/Game/Blueprints/MainMenuBluprints/CarMenuMode.RedrawWidget` _ascar_menu_mode)
    (`GameplayStatics.PlaySound2D` "/Game/Audio/MenuAudio/menu_Cue.menu_Cue" 1.0 1.0 0.0 null null)
    (bind _output_get (set `self.CursorPosition` (- (`self.CursorPosition`) 1)))
    (if (< _output_get 0)
      (set `self.CursorPosition` 4)
      (goto _label)
      (else
        (goto _label)))))

(event `InputAction|Right`
  (params (Key :type "Key Structure"))
  (:`Pressed`
    (bind _ascar_menu_mode (cast `/Game/Blueprints/MainMenuBluprints/CarMenuMode` (`GameplayStatics.GetGameMode`)))
    (`/Game/Blueprints/MainMenuBluprints/CarMenuMode.RedrawWidget` _ascar_menu_mode)
    (`GameplayStatics.PlaySound2D` "/Game/Audio/MenuAudio/menu_Cue.menu_Cue" 1.0 1.0 0.0 null null)
    (bind _result (`/Engine/EditorBlueprintResources/StandardMacros.IncrementInt` (`self.CursorPosition`))
      (:`  `
        (bind _output_get (set `self.CursorPosition` _result))
        (if (> _output_get 4)
          (set `self.CursorPosition` 0)
          (goto _label)
          (else
            (goto _label)))))))

(fn `UserConstructionScript`)