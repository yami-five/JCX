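; Player controller for the car game that handles restart and exit to the main menu, saving run stats before each.
; SaveStats loads the "CarSave" slot and writes a new save object with the higher score, accumulated wreck, pill and bottle totals, and the game mode's chosen car.
; Saving is skipped if no existing save loads.
; Restart waits briefly, saves, then calls RestartGame on CarGameMode, while Escape saves and opens MainMenu.
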(event `SaveStats`
  (bind _returnvalue (`GameplayStatics.LoadGameFromSlot` "CarSave"))
  (bind _ascar_save_game (cast `/Game/Blueprints/CarSaveGame` _returnvalue))
  (bind _ascar_game_pawn (cast `/Game/Blueprints/CarGamePawn` (`GameplayStatics.GetPlayerPawn` 0)))
  (bind _ascar_game_mode (cast `/Game/Blueprints/CarGameMode` (`GameplayStatics.GetGameMode`)))
  (bind _returnvalue_2 (`GameplayStatics.CreateSaveGameObject` "/Game/Blueprints/CarSaveGame.CarSaveGame_C"))
  (bind _output_get (set `self.SaveRef` _returnvalue_2))
  (bind _points (`/Game/Blueprints/CarGamePawn.Points` _ascar_game_pawn))
  (bind _highscore (`/Game/Blueprints/CarSaveGame.HighScore` _ascar_save_game))
  (if (> _points _highscore)
    (set `/Game/Blueprints/CarSaveGame.HighScore` _points _output_get)
    (else
      (set `/Game/Blueprints/CarSaveGame.HighScore` _highscore _output_get)))
  (set `/Game/Blueprints/CarSaveGame.CrashedCars` (+ (`/Game/Blueprints/CarSaveGame.CrashedCars` _ascar_save_game) (`/Game/Blueprints/CarGamePawn.TotalCarsWrecked` _ascar_game_pawn)) _output_get)
  (set `/Game/Blueprints/CarSaveGame.TotalPillsNum` (+ (`/Game/Blueprints/CarSaveGame.TotalPillsNum` _ascar_save_game) (`/Game/Blueprints/CarGamePawn.TotalPills` _ascar_game_pawn)) _output_get)
  (set `/Game/Blueprints/CarSaveGame.TotalBottlesNum` (+ (`/Game/Blueprints/CarSaveGame.TotalBottlesNum` _ascar_save_game) (`/Game/Blueprints/CarGamePawn.TotalItems` _ascar_game_pawn)) _output_get)
  (set `/Game/Blueprints/CarSaveGame.ChosenCar` (`/Game/Blueprints/CarGameMode.ChosenCar` _ascar_game_mode) _output_get)
  (`GameplayStatics.SaveGameToSlot` _output_get "CarSave"))

(event `InputAction|Restart`
  (params (Key :type "Key Structure"))
  (:`Pressed`
    (`KismetSystemLibrary.Delay` 0.2)
    (`self.SaveStats`)
    (bind _ascar_game_mode (cast `/Game/Blueprints/CarGameMode` (`GameplayStatics.GetGameMode`)))
    (`/Game/Blueprints/CarGameMode.RestartGame` _ascar_game_mode)))

(event `InputAction|Escape`
  (params (Key :type "Key Structure"))
  (:`Pressed`
    (`self.SaveStats`)
    (`GameplayStatics.OpenLevel` "MainMenu")))

(fn `UserConstructionScript`)